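; BP_Bullet is a projectile actor that flies in the direction the player pawn faces when it spawns.
; BeginPlay stores that forward vector, scaled, as a fixed step.
; Each Tick moves the actor by the step from its Sphere's location, with no sweep or delta-time scaling.
; It destroys itself once outside a per-axis distance tolerance around the player pawn's current location.
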(event `self.ReceiveBeginPlay`
  (bind _output_get (set `self.Rot` (* (`KismetMathLibrary.Conv_RotatorToVector` (`self.K2_GetActorRotation` (`GameplayStatics.GetPlayerPawn` 0))) 50))))

(event `self.ReceiveTick`
  (params (DeltaSeconds :type "Float (single-precision)"))
  (bind _returnvalue (`SceneComponent.K2_GetComponentLocation` (`self.Sphere`)))
  (if (== (`self.K2_GetActorLocation` (`GameplayStatics.GetPlayerPawn` 0)) _returnvalue :`ErrorTolerance` 12000.0)
    (`self.K2_SetActorLocation` (+ _returnvalue (stale `self.ReceiveBeginPlay` _output_get)))
    (else
      (`self.K2_DestroyActor`))))

(fn `UserConstructionScript`)