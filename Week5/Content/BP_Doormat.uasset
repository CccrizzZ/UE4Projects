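; BP_Doormat is a trigger actor that opens and closes a referenced door.
; Any overlap with its Cube component opens DoorRef, and ending the overlap closes it after a short retriggerable delay, which re-entry does not cancel.
; Separate actor-level overlap events print greeting and farewell debug text only for the player character.
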(event `self.ReceiveActorBeginOverlap`
  (params (OtherActor :type "Actor Object Reference"))
  (if (== OtherActor (`GameplayStatics.GetPlayerCharacter` 0))
    (`KismetSystemLibrary.PrintString` "Hello")))

(event `self.ReceiveActorEndOverlap`
  (params (OtherActor :type "Actor Object Reference"))
  (if (== OtherActor (`GameplayStatics.GetPlayerCharacter` 0))
    (`KismetSystemLibrary.PrintString` "Bye")))

(event `self.Cube.OnComponentEndOverlap`
  (params (OverlappedComponent :type "PrimitiveComponent Object Reference") (OtherActor :type "Actor Object Reference") (OtherComp :type "PrimitiveComponent Object Reference") (OtherBodyIndex :type Integer))
  (`KismetSystemLibrary.PrintString` "End Overlap")
  (`KismetSystemLibrary.RetriggerableDelay` 2.0)
  (`/Game/BP_Door.CloseDoor` (`self.DoorRef`)))

(event `self.Cube.OnComponentBeginOverlap`
  (params (OverlappedComponent :type "PrimitiveComponent Object Reference") (OtherActor :type "Actor Object Reference") (OtherComp :type "PrimitiveComponent Object Reference") (OtherBodyIndex :type Integer) (bFromSweep :type Boolean) (SweepResult :type "HitResult Structure (by ref)"))
  (`KismetSystemLibrary.PrintString` "Begin Overlap")
  (`/Game/BP_Door.OpenDoor` (`self.DoorRef`)))

(fn `UserConstructionScript`)