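; Door actor that swings its Cube mesh between a closed and an open rotation through OpenDoor and CloseDoor events.
; OpenDoor snaps the Cube open instantly, with no interpolation.
; CloseDoor resets the rotation only when the PlayerDetector volume overlaps no actors, otherwise rechecking after a retriggerable delay until it is clear.
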(event `CloseDoor`
  (if (== (`KismetArrayLibrary.Array_Length` (`self.GetOverlappingActors` (`self.PlayerDetector`) null)) 0) :!label _label
    (`SceneComponent.K2_SetRelativeRotation` (`self.Cube`) (struct) false false)
    (else
      (`KismetSystemLibrary.RetriggerableDelay` 2.0)
      (goto _label))))

(event `OpenDoor`
  (`SceneComponent.K2_SetRelativeRotation` (`self.Cube`) (struct :`Yaw` -85.0) false false))

(fn `UserConstructionScript`)