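; BP_Printer is an input test actor that prints messages to show when input actions fire.
; On BeginPlay it enables input from player controller 0.
; Releasing PrintText prints the key's display name in a release message.
; Pressing PrintAxis prints a fixed "Print Axis (val)" label behind a zero-equals-zero check that always passes, so no axis value is read.
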(event `self.ReceiveBeginPlay`
  (`self.EnableInput` (`GameplayStatics.GetPlayerController` 0)))

(event `InputAction|PrintText` :consume false
  (params (Key :type "Key Structure"))
  (:`Released`
    (`KismetSystemLibrary.PrintString` (`KismetStringLibrary.Concat_StrStr` "Hi! " (`KismetTextLibrary.Conv_TextToString` (`KismetInputLibrary.Key_GetDisplayName` Key)) " was released"))))

(event `InputAction|PrintAxis` :consume false
  (params (Key :type "Key Structure"))
  (:`Pressed`
    (if (`KismetMathLibrary.NearlyEqual_FloatFloat` 0.0)
      (`KismetSystemLibrary.PrintText` (`|FormatText` "Print Axis (val)")))))

(fn `UserConstructionScript`)